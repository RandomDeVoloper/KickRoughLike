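; BP_Soul is a soul pickup that awards XP when the player touches its Sphere, then destroys itself.
; Entering DetectRange starts a looping timer that interpolates the soul toward the player, cleared on exit or collection.
; UpdownAnim plays a timeline that moves the Soul component for a floating effect.
; DetectRangeUpdate enlarges the detection radius and starts another looping magnet timer whose handle is not stored.
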(event `self.Sphere.OnComponentBeginOverlap`
  (params (OverlappedComponent :type "PrimitiveComponent Object Reference") (OtherActor :type "Actor Object Reference") (OtherComp :type "PrimitiveComponent Object Reference") (OtherBodyIndex :type Integer) (bFromSweep :type Boolean) (SweepResult :type "HitResult Structure (by ref)"))
  ; Ruh toplama ve xp kazanma
  (if (== OtherActor (`GameplayStatics.GetPlayerCharacter` 0))
    (message `/Game/Mob/Interface/BPI_GameInteractions.AddXP` OtherActor 150)
    (`KismetSystemLibrary.Delay` 0.1)
    (`KismetSystemLibrary.K2_ClearAndInvalidateTimerHandle` (`self.MagnetTimerHandle`))
    (`self.K2_DestroyActor`)))

(event `UpdownAnim`
  ; Uçma animasyonu
  (bind (_direction _updown) (`Timeline|UpDown` :!via `PlayFromStart`)
    (:`Update`
      (`SceneComponent.K2_SetRelativeLocation` (`self.Soul`) _updown false false))))

(event `StartMagnetMovement`
  ; Eğer detect range e girerse karaktere doğru hareket etme end overlap oluncaysa timer sıfırlanır
  (`self.K2_SetActorLocation` (`KismetMathLibrary.VInterpTo` (`self.K2_GetActorLocation` self) (`self.K2_GetActorLocation` (`GameplayStatics.GetPlayerCharacter` 0)) 0.03 10.0)))

(event `self.DetectRange.OnComponentBeginOverlap`
  (params (OverlappedComponent :type "PrimitiveComponent Object Reference") (OtherActor :type "Actor Object Reference") (OtherComp :type "PrimitiveComponent Object Reference") (OtherBodyIndex :type Integer) (bFromSweep :type Boolean) (SweepResult :type "HitResult Structure (by ref)"))
  ; Eğer detect range e girerse karaktere doğru hareket etme end overlap oluncaysa timer sıfırlanır
  (if (== OtherActor (`GameplayStatics.GetPlayerCharacter` 0))
    (bind _returnvalue (`KismetSystemLibrary.K2_SetTimerDelegate` (delegate `StartMagnetMovement`) 0.03 true))
    (set `self.MagnetTimerHandle` _returnvalue)))

(event `self.DetectRange.OnComponentEndOverlap`
  (params (OverlappedComponent :type "PrimitiveComponent Object Reference") (OtherActor :type "Actor Object Reference") (OtherComp :type "PrimitiveComponent Object Reference") (OtherBodyIndex :type Integer))
  ; Eğer detect range e girerse karaktere doğru hareket etme end overlap oluncaysa timer sıfırlanır
  (if (== OtherActor (`GameplayStatics.GetPlayerCharacter` 0))
    (`KismetSystemLibrary.K2_ClearAndInvalidateTimerHandle` (`self.MagnetTimerHandle`))))

(event `DetectRangeUpdate`
  (bind _detectrange (`self.DetectRange`))
  (`SphereComponent.SetSphereRadius` _detectrange (* (`SphereComponent.SphereRadius` _detectrange) 1.1) true)
  (`KismetSystemLibrary.K2_SetTimerDelegate` (delegate `StartMagnetMovement`) 1.0 true))

(fn `UserConstructionScript`)