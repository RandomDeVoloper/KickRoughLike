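; Enemy actor that can be kicked and, once at zero health, becomes a ragdoll projectile that damages other enemies.
; OnKicked applies a fire overlay and, at zero health, launches the physics mesh and marks it deadly for a bouncing window.
; Mesh hits during that window damage other enemies and chain OnKicked onto them.
; Afterwards it awards player XP, spawns a BP_Soul and destroys itself; OnKickedMacro duplicates this death sequence.
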(event `OnKicked`
  (params (HitDirection :type "Vector Structure"))
  ;[0 0.006834 0.15 0.5] TEKME YİYİNCE ENEMY SEKMESİ
  (`MeshComponent.SetOverlayMaterial` (`self.Mesh`) "/Game/Itadori_aura/Material/MI_KickFire.MI_KickFire")
  (if (== (`self.CurrentEnemyHealth`) 0.0)
    (`PrimitiveComponent.SetCollisionEnabled` (`self.CapsuleComponent`) "NoCollision")
    (set `self.bIsDeadly` true)
    (`PrimitiveComponent.SetCollisionEnabled` (`self.Mesh`) "QueryAndPhysics")
    (`PrimitiveComponent.SetSimulatePhysics` (`self.Mesh`) true)
    (`GameplayStatics.PlaySound2D` "/Game/Mob/Sound/S_KickN1.S_KickN1" (`KismetMathLibrary.RandomFloatInRange` (`self.MinVolM`) (`self.MaxVolM`)) (`KismetMathLibrary.RandomFloatInRange` (`self.MaxVolM`) (`self.MaxPitchM`)) 0.0 "/Game/Mob/Sound/SC_Rule.SC_Rule" null)
    (`PrimitiveComponent.AddImpulse` (`self.Mesh`) (* HitDirection 50000) "pelvis" true)
    (`KismetSystemLibrary.Delay` (`self.BouncingTime`))
    (set `self.bIsDeadly` false)
    (message `/Game/Mob/Interface/BPI_GameInteractions.AddXP` (`GameplayStatics.GetPlayerCharacter` 0) (`self.BounceXPAmount`))
    (`KismetSystemLibrary.Delay` (`self.DestroyDuration`))
    (`KismetSystemLibrary.Delay` 0.01)
    (bind _returnvalue (`|SpawnActorFromClass` "/Game/Mob/EnemyBP/BP_Soul.BP_Soul_C" (`self.GetTransform`) "AdjustIfPossibleButAlwaysSpawn" "MultiplyWithRoot" null null))
    (`/Game/Mob/EnemyBP/BP_Soul.UpdownAnim` _returnvalue)
    (`/Game/Mob/EnemyBP/BP_Soul.DetectRangeUpdate` _returnvalue)
    (`self.K2_DestroyActor`)))

(event `self.Mesh.OnComponentHit`
  (params (HitComponent :type "PrimitiveComponent Object Reference") (OtherActor :type "Actor Object Reference") (OtherComp :type "PrimitiveComponent Object Reference") (NormalImpulse :type "Vector Structure") (Hit :type "HitResult Structure (by ref)"))
  ;[0 0.006834 0.15 0.5] Bouncing(enemylerin sekmesi)
  ;;[0.4678 0 0.02265] 1.cast
  (bind _asbp_enemy (cast `/Game/Mob/EnemyBP/BP_Enemy` OtherActor))
  (if (`self.bIsDeadly`)
    (bind _output_get (set `/Game/Mob/EnemyBP/BP_Enemy.CurrentEnemyHealth` (- (`/Game/Mob/EnemyBP/BP_Enemy.CurrentEnemyHealth` _asbp_enemy) 20.0) _asbp_enemy))
    ;;[0.4678 0 0.02265] 2.cast
    (bind _aswbp_hp_hud (cast `/Game/Mob/AugmentChoice/Widget/Enemy/WBP_HpHUD` (`WidgetComponent.GetUserWidgetObject` (`self.HealthBarW`))))
    (`/Game/Mob/AugmentChoice/Widget/Enemy/WBP_HpHUD.UpdateHealBar` _aswbp_hp_hud _output_get (`self.MaxEnemyHealth`))
    (`SceneComponent.SetVisibility` (`/Game/Mob/EnemyBP/BP_Enemy.HealthBarW` _asbp_enemy) false false)
    (`self.OnKicked` _asbp_enemy (* (`self.GetVelocity`) (`self.HitDirection`)))
    (`GameplayStatics.PlaySound2D` "/Game/Mob/Sound/S_KickN.S_KickN" (`KismetMathLibrary.RandomFloatInRange` 1.2 1.5) (`KismetMathLibrary.RandomFloatInRange` (`self.MinPitchM`) (`self.MaxPitchM`)) 0.0 "/Game/Mob/Sound/SC_Rule.SC_Rule" null)
    (message `/Game/Mob/Interface/BPI_GameInteractions.I_ReportHit` (`GameplayStatics.GetPlayerCharacter` 0))
    ;;[0.4678 0 0.02265] 3.cast
    (bind _aswbp_hp_hud_2 (cast `/Game/Mob/AugmentChoice/Widget/Enemy/WBP_HpHUD` (`WidgetComponent.GetUserWidgetObject` (`self.HealthBarW`))))
    (`/Game/Mob/AugmentChoice/Widget/Enemy/WBP_HpHUD.UpdateHealBar` _aswbp_hp_hud_2 _output_get (`self.MaxEnemyHealth`))))

(fn `HealthBar`
  (params (CurrentHealth :type "Float (single-precision)" :default 20.0) (MaxHealth :type "Float (double-precision)" :default 20.0))
  (bind _aswbp_hp_hud (cast `/Game/Mob/AugmentChoice/Widget/Enemy/WBP_HpHUD` (`WidgetComponent.GetUserWidgetObject` (`self.HealthBarW`))))
  (`/Game/Mob/AugmentChoice/Widget/Enemy/WBP_HpHUD.UpdateHealBar` _aswbp_hp_hud CurrentHealth MaxHealth))

(fn `UserConstructionScript`)

(fn `WalkAnim`
  (params (Enemy :type "Actor Object Reference"))
  (returns (SM_Enemy :type "SkeletalMeshComponent Object Reference") (Enemys :type "/Game/Mob/EnemyBP/BP_Enemy Object Reference"))
  (return null null))