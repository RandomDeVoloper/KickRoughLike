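; BP_Spawner is an enemy spawner that continuously spawns BP_Enemy pawns running BT_Enemy at its own location, using the player pawn's rotation.
; BeginPlay triggers AISpawner, which spawns an enemy and re-arms a looping timer on itself.
; Each pass shortens Duration after setting the timer, so spawning accelerates, with no clamp in the graph.
; The DoOnce resets immediately, and the next-stage message is unconnected.
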(event `AISpawner`
  (`/Engine/EditorBlueprintResources/StandardMacros.DoOnce` false :!label _label
    (:`Completed`
      (`AIBlueprintHelperLibrary.SpawnAIFromClass` "/Game/Mob/Enemy/BP_Enemy.BP_Enemy_C" "/Game/Mob/AI/BeheviorTree/BT_Enemy.BT_Enemy" (`self.K2_GetActorLocation` self) (`self.K2_GetActorRotation` (`GameplayStatics.GetPlayerPawn` 0)) false null)
      (`KismetSystemLibrary.K2_SetTimerDelegate` (delegate `AISpawner`) (`self.Duration`) true)
      (bind _output_get (set `self.Duration` (- (`self.Duration`) 0.1)))
      (`KismetSystemLibrary.PrintString` (`KismetStringLibrary.Conv_DoubleToString` _output_get))
      (goto _label :!via `Reset`))))

(event `self.ReceiveBeginPlay`
  (`self.AISpawner`))

(event `SetTimer`)

(fn `UserConstructionScript`)